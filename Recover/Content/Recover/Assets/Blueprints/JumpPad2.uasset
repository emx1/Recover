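; JumpPad2 is a jump pad actor that throws the first-person character into the air on contact.
; Overlapping its ScrabbleLetter component casts the other actor to FirstPersonCharacter and switches its movement mode to Falling.
; It then overwrites the movement velocity directly, without LaunchCharacter, combining a strong fixed upward boost with a small horizontal push along the player camera's facing.
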(event `self.ScrabbleLetter.OnComponentBeginOverlap`
  (params (OverlappedComponent :type "PrimitiveComponent Object Reference") (OtherActor :type "Actor Object Reference") (OtherComp :type "PrimitiveComponent Object Reference") (OtherBodyIndex :type Integer) (bFromSweep :type Boolean) (SweepResult :type "HitResult Structure (by ref)"))
  (bind _returnvalue (`GameplayStatics.GetPlayerCameraManager` 0))
  (bind _asfirst_person_character (cast `/Game/FirstPersonBP/Blueprints/FirstPersonCharacter` OtherActor))
  (bind _charactermovement (`Character.CharacterMovement` _asfirst_person_character))
  (`CharacterMovementComponent.SetMovementMode` _charactermovement "MOVE_Falling" 0)
  (set `MovementComponent.Velocity` (`KismetMathLibrary.MakeVector` (* (.x (`self.GetActorForwardVector` _returnvalue)) 100.0) (* (.y (`KismetMathLibrary.Conv_RotatorToVector` (`self.K2_GetActorRotation` _returnvalue))) 100.0) 1500.0) _charactermovement))

(fn `UserConstructionScript`)