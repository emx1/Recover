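; JumpPad Blueprint meant to change the first-person player's jump velocity around a Box trigger.
; On end overlap, it sets the player's JumpZVelocity to NormalJumpHeight.
; The logic that saves the current velocity and applies JumpHeight is disconnected, and begin overlap is empty.
; As wired, the pad never applies its boost and restores a value it never captured.
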(event `self.Box.OnComponentBeginOverlap`
  (params (OverlappedComponent :type "PrimitiveComponent Object Reference") (OtherActor :type "Actor Object Reference") (OtherComp :type "PrimitiveComponent Object Reference") (OtherBodyIndex :type Integer) (bFromSweep :type Boolean) (SweepResult :type "HitResult Structure (by ref)")))

(event `self.Box.OnComponentEndOverlap`
  (params (OverlappedComponent :type "PrimitiveComponent Object Reference") (OtherActor :type "Actor Object Reference") (OtherComp :type "PrimitiveComponent Object Reference") (OtherBodyIndex :type Integer))
  (if (== OtherActor (`GameplayStatics.GetPlayerCharacter` 0))
    (bind _asfirst_person_character (cast `/Game/FirstPersonBP/Blueprints/FirstPersonCharacter` OtherActor))
    (set `CharacterMovementComponent.JumpZVelocity` (`self.normalJumpHeight`) (`Character.CharacterMovement` _asfirst_person_character))))

(fn `UserConstructionScript`)