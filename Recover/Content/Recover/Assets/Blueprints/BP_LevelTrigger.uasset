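; BP_LevelTrigger is a trigger volume that becomes interactable when the first-person character stands inside it carrying enough pickups.
; Box overlaps track presence and, on entry, latch EnoughPickups once the character's Pickups count reaches NumberOfPickups.
; Tick derives CanInteract from both flags.
; The Interact input only sets InteractPressed and prints, while Response is a debug print stub, so no level action happens here.
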(event `self.Box.OnComponentBeginOverlap`
  (params (OverlappedComponent :type "PrimitiveComponent Object Reference") (OtherActor :type "Actor Object Reference") (OtherComp :type "PrimitiveComponent Object Reference") (OtherBodyIndex :type Integer) (bFromSweep :type Boolean) (SweepResult :type "HitResult Structure (by ref)"))
  (bind _asfirst_person_character (cast `/Game/FirstPersonBP/Blueprints/FirstPersonCharacter` OtherActor))
  (set `self.inTrigger` true)
  (if (>= (`KismetArrayLibrary.Array_Length` (`/Game/FirstPersonBP/Blueprints/FirstPersonCharacter.Pickups` _asfirst_person_character)) (`self.numberOfPickups`))
    (set `self.enoughPickups` true)
    (`KismetSystemLibrary.PrintString` (`KismetStringLibrary.Conv_IntToString` 0))))

(event `self.Box.OnComponentEndOverlap`
  (params (OverlappedComponent :type "PrimitiveComponent Object Reference") (OtherActor :type "Actor Object Reference") (OtherComp :type "PrimitiveComponent Object Reference") (OtherBodyIndex :type Integer))
  (cast `/Game/FirstPersonBP/Blueprints/FirstPersonCharacter` OtherActor)
  (set `self.inTrigger` false))

(event `InputAction|Interact`
  (params (Key :type "Key Structure" :default "AnyKey"))
  (:`Pressed`
    (set `self.interactPressed` true)
    (`KismetSystemLibrary.PrintString` "Interact Pressed")))

(event `self.ReceiveTick`
  (params (DeltaSeconds :type "Float (single-precision)"))
  (if (`self.inTrigger`)
    (if (`self.enoughPickups`)
      (set `self.canInteract` true)
      (else
        (set `self.canInteract` false :!label _label)))
    (else
      (goto _label))))

(fn `Response`
  (`KismetSystemLibrary.PrintString` "Delay Worked!"))

(fn `UserConstructionScript`)